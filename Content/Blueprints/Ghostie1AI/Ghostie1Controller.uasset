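; AI controller for the Ghostie1Character pawn that chooses which ghost behavior tree to run.
; On BeginPlay it casts the controlled pawn and branches on the character's Num variable to start Ghostie1BT, Ghostie3BT or Ghostie4BT.
; A failed cast or any other Num value starts no tree, and the controller has no other logic.
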(event EventBeginPlay
  (bind _asghostie_1character (Utilities|Casting|CastToGhostie1Character (Pawn|GetControlledPawn)))
  (if (== (Variables|/Game/Blueprints/Ghostie1AI/Ghostie1Character.Ghostie1Character_C|GetNum _asghostie_1character) 0)
    (AI|RunBehaviorTree "/Game/Blueprints/Ghostie1AI/Ghostie1BT.Ghostie1BT")
    (elif (== (Variables|/Game/Blueprints/Ghostie1AI/Ghostie1Character.Ghostie1Character_C|GetNum _asghostie_1character) 1)
      (AI|RunBehaviorTree "/Game/Blueprints/Ghostie3AI/Ghostie3BT.Ghostie3BT")
      (elif (== (Variables|/Game/Blueprints/Ghostie1AI/Ghostie1Character.Ghostie1Character_C|GetNum _asghostie_1character) 2)
        (AI|RunBehaviorTree "/Game/Blueprints/Ghostie1AI/Ghostie4BT.Ghostie4BT")))))

(event EventTick
  (params (DeltaSeconds :type Float%20%28single-precision%29)))

(fn ConstructionScript)