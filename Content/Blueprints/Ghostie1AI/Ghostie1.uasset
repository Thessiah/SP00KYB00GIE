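; Ghostie1 is a ghost character that reacts to pawns it sees.
; Its PawnSensing component passes each seen pawn to CallAttackTarget, which hands the attack off to logic outside this graph.
; Tick and the construction script are empty.
; Disconnected leftover nodes hold an unused SeesPlayer flag with a timed reset and debug prints of Target and that flag.
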(event OnSeePawn(PawnSensing)
  (params (Pawn :type Pawn%20Object%20Reference))
  (Default|CallAttackTarget Pawn))

(event EventTick
  (params (DeltaSeconds :type Float%20%28single-precision%29))
  ;[1 1 1] Debug Print
)

(fn ConstructionScript)