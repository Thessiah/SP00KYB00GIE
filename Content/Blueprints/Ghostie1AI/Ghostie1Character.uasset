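; Ghostie1 enemy character, a ghost that is visible only while the first-person HUD's camera overlay is shown.
; Tick toggles its visibility, fires attack or don't-attack calls based on a 500-unit distance to the player, and debug-prints that distance.
; The HitGhostie event swaps its walking flag for a stunned one for four seconds.
; The PawnSensing handler is empty, leaving its older attack logic disconnected.
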(event OnSeePawn(PawnSensing)
  (params (Pawn :type Pawn%20Object%20Reference)))

(event Custom|HitGhostie_Event_0
  (Variables|Default|SetisStunned true)
  (Variables|Default|SetisWalking false)
  (Utilities|FlowControl|Delay 4.0)
  (Variables|Default|SetisStunned false)
  (Variables|Default|SetisWalking true))

(event EventBeginPlay
  (EventDispatchers|AssignHitGhostie (delegate Custom|HitGhostie_Event_0))
  (Variables|Default|SetisWalking true))

(event EventTick
  (params (DeltaSeconds :type Float%20%28single-precision%29))
  (bind _returnvalue (Game|GetPlayerCharacter 0))
  (bind _self self)
  (bind _returnvalue_2 (Transformation|GetActorLocation _returnvalue))
  (bind _returnvalue_3 (Transformation|GetActorLocation _self))
  (bind _returnvalue_4 (- _returnvalue_2 _returnvalue_3))
  (bind _returnvalue_5 (Math|Vector|VectorLength _returnvalue_4))
  (bind _asfirst_person_hud (Utilities|Casting|CastToFirstPersonHUD (HUD|GetHUD (Game|GetPlayerController 0))))
  (if (Variables|/Game/FirstPersonBP/Blueprints/FirstPersonHUD.FirstPersonHUD_C|GetShowCameraOverlay _asfirst_person_hud)
    (Rendering|SetActorHiddenInGame false)
    (else
      (Rendering|SetActorHiddenInGame true)))
  (if (<= _returnvalue_5 5e+02)
    (Default|CallAttackTarget _returnvalue)
    (else
      (Default|CallDontAttackTarget)))
  (Development|PrintString (Utilities|String|ToString(Float) _returnvalue_5)))

(fn ConstructionScript)