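; Ghostie enemy character that chases the player, can be stunned, and changes visibility with the player's camera overlay.
; Each Tick it swaps its body material between visible and translucent based on the HUD's camera overlay flag.
; It fires attack or stop-attack dispatchers based on whether a living player is within range.
; The hit event stuns it and halts walking for a few seconds; pawn-sensing logic is left disconnected.
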(event OnSeePawn(PawnSensing)
  (params (Pawn :type Pawn%20Object%20Reference)))

(event Custom|HitGhostie_Event_0
  (Variables|Default|SetisStunned true)
  (Variables|Default|SetisWalking false)
  (Utilities|FlowControl|Delay 4.0)
  (Variables|Default|SetisStunned false)
  (Variables|Default|SetisWalking true))

(event EventBeginPlay
  (EventDispatchers|AssignHitGhostie (delegate Custom|HitGhostie_Event_0))
  (Variables|Default|SetisWalking true))

(event EventTick
  (params (DeltaSeconds :type Float%20%28single-precision%29))
  (bind _returnvalue (Game|GetPlayerCharacter 0))
  (bind _asfirst_person_hud (Utilities|Casting|CastToFirstPersonHUD (HUD|GetHUD (Game|GetPlayerController 0))))
  (if (Variables|/Game/FirstPersonBP/Blueprints/FirstPersonHUD.FirstPersonHUD_C|GetShowCameraOverlay _asfirst_person_hud)
    (Rendering|Material|SetMaterial 0 "/Game/_Body_Visible._Body_Visible")
    (else
      (Rendering|Material|SetMaterial 0 "/Game/_BodyTRANS._BodyTRANS")))
  (bind _asfirst_person_character (Utilities|Casting|CastToFirstPersonCharacter _returnvalue))
  (if (and (<= (Math|Vector|VectorLength (- (Transformation|GetActorLocation _returnvalue) (Transformation|GetActorLocation self))) 6e+02) (not (Variables|/Game/FirstPersonBP/Blueprints/FirstPersonCharacter.FirstPersonCharacter_C|GetisDead _asfirst_person_character)))
    (Default|CallAttackTarget _returnvalue)
    (else
      (Default|CallDontAttackTarget))))

(fn ConstructionScript)