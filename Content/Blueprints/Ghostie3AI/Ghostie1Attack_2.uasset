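; Behavior tree task for a ghost attack that costs the first-person player one Health.
; It calls the hit function on Ghostie1 or Ghostie2 pawns; other controllers skip straight to the damage step.
; If off cooldown, it flashes HUD damage alpha and plays a heartbeat sound.
; Delays started after FinishExecute restore that Health point and re-arm the attack.
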(event EventReceiveExecute
  (params (OwnerActor :type Actor%20Object%20Reference))
  (bind _returnvalue (Game|GetPlayerController 0))
  (bind _returnvalue_2 (HUD|GetHUD _returnvalue))
  (bind _asghostie_2controller (Utilities|Casting|CastToGhostie2Controller OwnerActor)
    (:then
      (bind _asghostie_2character (Utilities|Casting|CastToGhostie2Character (Pawn|GetControlledPawn _asghostie_2controller)))
      (Default|CallHitGhostie2 _asghostie_2character))
    (:CastFailed
      (bind _asghostie_1controller (Utilities|Casting|CastToGhostie1Controller OwnerActor)
        (:then
          (bind _asghostie_1character (Utilities|Casting|CastToGhostie1Character (Pawn|GetControlledPawn _asghostie_1controller)))
          (Default|CallHitGhostie _asghostie_1character))
        (:CastFailed
          _))))
  (if (Variables|Default|GetcanAttack)
    (Variables|Default|SetcanAttack false)
    (bind _asfirst_person_hud (Utilities|Casting|CastToFirstPersonHUD _returnvalue_2))
    (Variables|/Game/FirstPersonBP/Blueprints/FirstPersonHUD.FirstPersonHUD_C|SetAlphaDmg _asfirst_person_hud 1.0)
    (Audio|PlaySoundatLocation "/Game/Audio/heartbeat.heartbeat" (Transformation|GetActorLocation _returnvalue_2))
    (bind _asfirst_person_character (Utilities|Casting|CastToFirstPersonCharacter (Game|GetPlayerCharacter 0)))
    (Variables|/Game/FirstPersonBP/Blueprints/FirstPersonCharacter.FirstPersonCharacter_C|SetHealth _asfirst_person_character (- (Variables|/Game/FirstPersonBP/Blueprints/FirstPersonCharacter.FirstPersonCharacter_C|GetHealth _asfirst_person_character) 1))
    (AI|BehaviorTree|FinishExecute true)
    (Utilities|FlowControl|Sequence
      (:then_0
        (Utilities|FlowControl|Delay 15.0)
        (Variables|/Game/FirstPersonBP/Blueprints/FirstPersonCharacter.FirstPersonCharacter_C|SetHealth _asfirst_person_character (+ (Variables|/Game/FirstPersonBP/Blueprints/FirstPersonCharacter.FirstPersonCharacter_C|GetHealth _asfirst_person_character) 1)) ; Regen this health 10s later
      )
      (:then_1
        (Utilities|FlowControl|Delay 4.0)
        (Variables|Default|SetcanAttack true)))
    (else
      (AI|BehaviorTree|FinishExecute true))))