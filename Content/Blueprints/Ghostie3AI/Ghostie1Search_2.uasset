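; Behavior tree node, apparently a service, that relays Ghostie1Character events into the Ghostie AI's blackboard.
; On activation it binds to the controlled character's attack, stop-attack and hit dispatchers.
; An attack event stores the target player and its distance at that moment, while a stop event clears the target.
; A hit sets the Stunned key, then clears it after a fixed delay.
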(event Custom|HitGhostie_Event_0
  (Class|BTFunctionLibrary|SetBlackboardValueasBool (Variables|Default|GetStunned) true)
  (Utilities|FlowControl|Delay 4.0)
  (Class|BTFunctionLibrary|SetBlackboardValueasBool (Variables|Default|GetStunned) false))

(event Custom|AttackTarget_Event_0
  (params (Player :type Actor%20Object%20Reference))
  (Class|BTFunctionLibrary|SetBlackboardValueasObject (Variables|Default|GetTargetPlayer) Player)
  (Class|BTFunctionLibrary|SetBlackboardValueasFloat (Variables|Default|GetTargetDistance) (Transformation|GetDistanceTo Player (Pawn|GetControlledPawn (stale EventReceiveActivation _asghostie_1controller)))))

(event Custom|DontAttackTarget_Event_0
  (Class|BTFunctionLibrary|SetBlackboardValueasObject (Variables|Default|GetTargetPlayer)))

(event EventReceiveActivation
  (params (OwnerActor :type Actor%20Object%20Reference))
  (bind _asghostie_1controller (Utilities|Casting|CastToGhostie1Controller OwnerActor))
  (bind _asghostie_1character (Utilities|Casting|CastToGhostie1Character (Pawn|GetControlledPawn _asghostie_1controller)))
  (EventDispatchers|BindEventtoAttackTarget _asghostie_1character (delegate Custom|AttackTarget_Event_0))
  (EventDispatchers|AssignDontAttackTarget _asghostie_1character (delegate Custom|DontAttackTarget_Event_0))
  (EventDispatchers|AssignHitGhostie _asghostie_1character (delegate Custom|HitGhostie_Event_0)))