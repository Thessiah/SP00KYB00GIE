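; Key-locked swinging door that the player opens and closes with E while inside its trigger volume, which enables input.
; E checks the first-person character's first KeyArray slot, then either plays a locked sound or toggles the door, guarded by IsMoving.
; The DoorMovement timeline drives yaw relative to the rotation saved at construction.
; Actor overlap flags the character as touching and shows a prompt widget until E is first pressed.
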(event OnComponentBeginOverlap(TriggerVolume)
  (params (OtherActor :type Actor%20Object%20Reference) (OtherComp :type Primitive%20Component%20Object%20Reference) (OtherBodyIndex :type Integer) (bFromSweep :type Boolean) (SweepResult :type Hit%20Result%20Structure%20%28by%20ref%29))
  (Input|EnableInput (Game|GetPlayerController 0))
  (Utilities|FlowControl|Gate true) ; enters at Open
)

(event OnComponentEndOverlap(TriggerVolume)
  (params (OtherActor :type Actor%20Object%20Reference) (OtherComp :type Primitive%20Component%20Object%20Reference) (OtherBodyIndex :type Integer))
  (Input|DisableInput (Game|GetPlayerController 0)))

(event EventActorBeginOverlap
  (params (OtherActor :type Actor%20Object%20Reference))
  ;[1 1 1] Collision with Player, show UI
  (bind _asfirst_person_character (Utilities|Casting|CastToFirstPersonCharacter OtherActor))
  (Variables|/Game/FirstPersonBP/Blueprints/FirstPersonCharacter.FirstPersonCharacter_C|SetTouchingDoor _asfirst_person_character true)
  (if (not (Variables|Default|GetOpenedOnce)) ; Only show msg if first time
    (bind _returnvalue (UserInterface|CreateWidget "/Game/UI/DoorUI_BP.DoorUI_BP_C"))
    (Variables|/Game/UI/DoorUI_BP.DoorUI_BP_C|SetFirstDoor _returnvalue self)
    (UserInterface|Viewport|AddtoViewport _returnvalue 0)))

(event EventActorEndOverlap
  (params (OtherActor :type Actor%20Object%20Reference))
  ;[1 1 1] Collision with Player, show UI
  (bind _asfirst_person_character (Utilities|Casting|CastToFirstPersonCharacter OtherActor))
  (Variables|/Game/FirstPersonBP/Blueprints/FirstPersonCharacter.FirstPersonCharacter_C|SetTouchingDoor _asfirst_person_character false)
  (Widget|RemovefromParent (stale EventActorBeginOverlap _returnvalue)))

(event Input|KeyboardEvents|E
  (:Pressed
    (Utilities|FlowControl|Gate true
      (:Exit
        (Variables|Default|SetOpenedOnce true)
        (Widget|RemovefromParent (stale EventActorBeginOverlap _returnvalue))
        (bind _asfirst_person_character (Utilities|Casting|CastToFirstPersonCharacter (Game|GetPlayerCharacter 0)))
        (if (Utilities|Array|Get(acopy) (Variables|/Game/FirstPersonBP/Blueprints/FirstPersonCharacter.FirstPersonCharacter_C|GetKeyArray _asfirst_person_character))
          (if (not (Variables|Default|GetIsMoving))
            (Variables|Default|SetIsMoving true)
            (if (Variables|Default|GetIsOpen)
              (Variables|Default|SetIsOpen false)
              (Audio|PlaySoundatLocation "/Game/FirstPersonBP/Audio/door_open.door_open" "0, 0, 0")
              (bind _doorrotation (Timeline|DoorMovement ReverseFromEnd)
                (:Update
                  (Transformation|SetActorRelativeRotation (Class|KismetMathLibrary|MakeRot 0.0 (+ _doorrotation (.yaw (Variables|Default|GetInitialRotation))) 0.0))
                  (Utilities|FlowControl|Delay 1.1)
                  (Variables|Default|SetIsMoving false)))
              (else
                (Variables|Default|SetIsOpen true)
                (Audio|PlaySoundatLocation "/Game/FirstPersonBP/Audio/door_close.door_close" "0, 0, 0")
                (Timeline|DoorMovement PlayFromStart))))
          (else
            (Audio|PlaySoundatLocation "/Game/External_Assets/door-lock-1.door-lock-1" (Transformation|GetActorLocation))))))))

(fn ConstructionScript
  (bind _returnvalue (Transformation|GetActorRotation))
  (Transformation|SetActorRotation _returnvalue)
  (Variables|Default|SetInitialRotation _returnvalue))