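; Behavior tree node for the Ghostie2 enemy AI that feeds player-targeting and stun state into the blackboard.
; On activation it binds handlers to the character's attack, stop-attack and hit events.
; Attack events store the player and distance, with a forward line trace setting CanAttack only when it hits the first-person character.
; Stop-attack events clear the target, while hits set Stunned for a short delay.
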(event Custom|AttackTarget2_Event_0
  (params (Player :type Actor%20Object%20Reference))
  (bind _canattack (Variables|Default|GetcanAttack))
  (Class|BTFunctionLibrary|SetBlackboardValueasObject (Variables|Default|GetTargetPlayer) Player)
  (Class|BTFunctionLibrary|SetBlackboardValueasFloat (Variables|Default|GetTargetDistance) (Transformation|GetDistanceTo Player (Pawn|GetControlledPawn (stale EventReceiveActivation _asghostie_2controller))))
  (bind _outhit (Collision|LineTraceForObjects (+ (Transformation|GetActorLocation (stale EventReceiveActivation _asghostie_2character)) (* (Math|Vector|GetForwardVector (Transformation|GetActorRotation (stale EventReceiveActivation _asghostie_2character))) 1e+02)) (+ (Transformation|GetActorLocation (stale EventReceiveActivation _asghostie_2character)) (* (Math|Vector|GetForwardVector (Transformation|GetActorRotation (stale EventReceiveActivation _asghostie_2character))) 1.5e+03)) (Utilities|Array|MakeArray "ObjectTypeQuery1" "ObjectTypeQuery2" "ObjectTypeQuery3") false 0 "None"))
  (Utilities|Casting|CastToFirstPersonCharacter (.HitActor (Collision|BreakHitResult _outhit))
    (:then
      (Class|BTFunctionLibrary|SetBlackboardValueasBool _canattack true))
    (:CastFailed
      (Class|BTFunctionLibrary|SetBlackboardValueasBool _canattack false))))

(event Custom|DontAttackTarget2_Event_0
  (Class|BTFunctionLibrary|SetBlackboardValueasObject (Variables|Default|GetTargetPlayer)))

(event Custom|HitGhostie2_Event_0
  (Class|BTFunctionLibrary|SetBlackboardValueasBool (Variables|Default|GetStunned) true)
  (Utilities|FlowControl|Delay 3.0)
  (Class|BTFunctionLibrary|SetBlackboardValueasBool (Variables|Default|GetStunned) false))

(event EventReceiveActivation
  (params (OwnerActor :type Actor%20Object%20Reference))
  (bind _asghostie_2controller (Utilities|Casting|CastToGhostie2Controller OwnerActor))
  (bind _asghostie_2character (Utilities|Casting|CastToGhostie2Character (Pawn|GetControlledPawn _asghostie_2controller)))
  (EventDispatchers|AssignAttackTarget2 _asghostie_2character (delegate Custom|AttackTarget2_Event_0))
  (EventDispatchers|AssignDontAttackTarget2 _asghostie_2character (delegate Custom|DontAttackTarget2_Event_0))
  (EventDispatchers|AssignHitGhostie2 _asghostie_2character (delegate Custom|HitGhostie2_Event_0)))