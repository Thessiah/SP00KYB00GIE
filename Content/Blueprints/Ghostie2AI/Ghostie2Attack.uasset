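; Behavior tree task for the Ghostie2 AI that attacks the player on a short cooldown.
; An attack sets the HUD damage alpha, plays a heartbeat sound and takes one point of player health.
; It finishes immediately, then parallel delays re-enable attacking after 3 seconds and restore the health point after 15 seconds, despite a comment saying 10.
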(event EventReceiveExecute
  (params (OwnerActor :type Actor%20Object%20Reference))
  (bind _returnvalue (Game|GetPlayerController 0))
  (bind _returnvalue_2 (HUD|GetHUD _returnvalue))
  (if (Variables|Default|GetcanAttack)
    (Variables|Default|SetcanAttack false)
    (bind _asfirst_person_hud (Utilities|Casting|CastToFirstPersonHUD _returnvalue_2))
    (Variables|/Game/FirstPersonBP/Blueprints/FirstPersonHUD.FirstPersonHUD_C|SetAlphaDmg _asfirst_person_hud 1.0)
    (Audio|PlaySoundatLocation "/Game/Audio/heartbeat.heartbeat" (Transformation|GetActorLocation _returnvalue_2))
    (bind _asfirst_person_character (Utilities|Casting|CastToFirstPersonCharacter (Game|GetPlayerCharacter 0)))
    (Variables|/Game/FirstPersonBP/Blueprints/FirstPersonCharacter.FirstPersonCharacter_C|SetHealth _asfirst_person_character (- (Variables|/Game/FirstPersonBP/Blueprints/FirstPersonCharacter.FirstPersonCharacter_C|GetHealth _asfirst_person_character) 1))
    (AI|BehaviorTree|FinishExecute true)
    (Utilities|FlowControl|Sequence
      (:then_0
        (Utilities|FlowControl|Delay 15.0)
        (Variables|/Game/FirstPersonBP/Blueprints/FirstPersonCharacter.FirstPersonCharacter_C|SetHealth _asfirst_person_character (+ (Variables|/Game/FirstPersonBP/Blueprints/FirstPersonCharacter.FirstPersonCharacter_C|GetHealth _asfirst_person_character) 1)) ; Regen this health 10s later
      )
      (:then_1
        (Utilities|FlowControl|Delay 3.0)
        (Variables|Default|SetcanAttack true)))
    (else
      (AI|BehaviorTree|FinishExecute true))))