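; Character Blueprint for the Ghostie2 enemy, an AI ghost that reacts to the player's camera overlay and flashlight.
; Its HitGhostie2 event stuns it and clears the walking flag for a few seconds.
; Each Tick swaps its body material with the HUD camera overlay state.
; Tick also calls AttackTarget2 on the player while the flashlight is on and the player is alive, otherwise DontAttackTarget2.
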(event Custom|HitGhostie2_Event_0
  (Variables|Default|SetisStunned true)
  (Variables|Default|SetisWalking false)
  (Utilities|FlowControl|Delay 4.0)
  (Variables|Default|SetisStunned false)
  (Variables|Default|SetisWalking true))

(event EventBeginPlay
  (EventDispatchers|AssignHitGhostie2 (delegate Custom|HitGhostie2_Event_0))
  (Variables|Default|SetisWalking true))

(event EventTick
  (params (DeltaSeconds :type Float%20%28single-precision%29))
  (bind _returnvalue (Game|GetPlayerCharacter 0))
  (bind _asfirst_person_hud (Utilities|Casting|CastToFirstPersonHUD (HUD|GetHUD (Game|GetPlayerController 0))))
  (if (Variables|/Game/FirstPersonBP/Blueprints/FirstPersonHUD.FirstPersonHUD_C|GetShowCameraOverlay _asfirst_person_hud)
    (Rendering|Material|SetMaterial 0 "/Game/_Body._Body")
    (else
      (Rendering|Material|SetMaterial 0 "/Game/_BodyTRANS._BodyTRANS")))
  (bind _asfirst_person_character (Utilities|Casting|CastToFirstPersonCharacter _returnvalue))
  (if (and (Variables|/Game/FirstPersonBP/Blueprints/FirstPersonCharacter.FirstPersonCharacter_C|GetFlashlight _asfirst_person_character) (not (Variables|/Game/FirstPersonBP/Blueprints/FirstPersonCharacter.FirstPersonCharacter_C|GetisDead _asfirst_person_character)))
    (Default|CallAttackTarget2 _returnvalue)
    (else
      (Default|CallDontAttackTarget2))))

(fn ConstructionScript)