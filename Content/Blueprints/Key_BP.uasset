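; Key_BP is a collectible key actor that the first-person player can pick up.
; When the player character overlaps it and its PickupCone is among the overlapping components, it creates a KeyUI_BP widget referencing itself, then removes it when the overlap ends.
; Its Pickup function marks the slot at KeyNum in the character's KeyArray, destroys the actor and plays a pickup sound at its location.
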(event EventActorBeginOverlap
  (params (OtherActor :type Actor%20Object%20Reference))
  ;[1 1 1] Create UI widget on item hover
  (if (not (Variables|Default|GetShowingUI))
    (if (== OtherActor (Game|GetPlayerCharacter 0))
      (bind _asfirst_person_character (Utilities|Casting|CastToFirstPersonCharacter OtherActor))
      (if (Utilities|Array|ContainsItem (Class|Actor|GetOverlappingComponents) (Variables|/Game/FirstPersonBP/Blueprints/FirstPersonCharacter.FirstPersonCharacter_C|GetPickupCone _asfirst_person_character))
        (bind _returnvalue (UserInterface|CreateWidget "/Game/UI/KeyUI_BP.KeyUI_BP_C"))
        (Variables|/Game/UI/KeyUI_BP.KeyUI_BP_C|SetKey _returnvalue self)
        (UserInterface|Viewport|AddtoViewport _returnvalue 0)
        (Variables|Default|SetShowingUI true)))))

(event EventActorEndOverlap
  (params (OtherActor :type Actor%20Object%20Reference))
  ;[1 1 1] Hide UI widget
  (if (Variables|Default|GetShowingUI)
    (if (== OtherActor (Game|GetPlayerCharacter 0))
      (Widget|RemovefromParent (stale EventActorBeginOverlap _returnvalue))
      (Variables|Default|SetShowingUI false))))

(fn ConstructionScript)

(fn Pickup
  (bind _asfirst_person_character (Utilities|Casting|CastToFirstPersonCharacter (Game|GetPlayerCharacter 0)))
  (Utilities|Array|SetArrayElem (Variables|/Game/FirstPersonBP/Blueprints/FirstPersonCharacter.FirstPersonCharacter_C|GetKeyArray _asfirst_person_character) (Variables|Default|GetKeyNum) (Variables|Default|GetSetTrue))
  (Actor|DestroyActor)
  (Audio|PlaySoundatLocation "/Game/External_Assets/wine_bottle_pick_up_from_table.wine_bottle_pick_up_from_table" (Transformation|GetActorLocation)))